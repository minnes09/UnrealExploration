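; Battery pickup Blueprint that plays a lightning-drain effect toward the player character when collected.
; WasCollected spawns an electricity arc on the pickup mesh and targets whichever middle-finger bone, left or right, is nearer.
; A looping Delay keeps the beam endpoint on that hand, while a parallel one-second Delay defers the parent's WasCollected logic.
; An unconnected earlier version always targeting the right hand remains in the graph.
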(event EventBeginPlay)

(event Collision|EventActorBeginOverlap
  (params (OtherActor :type Actor%20Object%20Reference)))

(event EventTick
  (params (DeltaSeconds :type Float%20%28single-precision%29)))

(event EventWasCollected
  (bind _returnvalue (Game|GetPlayerCharacter 0))
  (bind _pickupmesh (Variables|Default|GetPickupMesh))
  (bind _returnvalue_2 (Transformation|GetSocketLocation _pickupmesh "None"))
  (bind _mesh (Variables|/Script/Engine.Character|GetMesh _returnvalue))
  (bind _returnvalue_3 (Class|SkinnedMeshComponent|GetSocketBoneName _mesh "middle_03_r"))
  (bind _returnvalue_4 (Class|SkinnedMeshComponent|GetSocketBoneName _mesh "middle_03_l"))
  (bind _returnvalue_5 (Effects|SpawnEmitterAttached "/Game/ExampleContent/Effects/ParticleSystems/P_electricity_arc.P_electricity_arc" (Variables|Default|GetPickupMesh) "None" "0, 0, 0" "0, 0, 0" "SnapToTargetIncludingScale"))
  ;[0.3474 0.9102 1] Set Socket with minimum distance
  (if (<= (Math|Vector|VectorLength (- (Transformation|GetSocketLocation _mesh _returnvalue_3) _returnvalue_2)) (Math|Vector|VectorLength (- _returnvalue_2 (Transformation|GetSocketLocation _mesh _returnvalue_4))))
    (Variables|Default|SetHand _returnvalue_3)
    (else
      (Variables|Default|SetHand _returnvalue_4)))
  ;[0.4818 0.4362 1] Capture Power with right hand
  (Class|ParticleSystemComponent|SetBeamTargetPoint _returnvalue_5 0 (Transformation|GetSocketLocation (Variables|/Script/Engine.Character|GetMesh (Game|GetPlayerCharacter 0)) (Variables|Default|GetHand)) :!label _label)
  (Utilities|FlowControl|Sequence
    (:then_0
      (Utilities|FlowControl|Delay 1.0)
      (|CallParentFunction))
    (:then_1
      (Utilities|FlowControl|Delay 0.05)
      (goto _label))))

(event Input|KeyboardEvents|1
  (params (Key :type Key%20Structure :default "AnyKey")))

(fn ConstructionScript)