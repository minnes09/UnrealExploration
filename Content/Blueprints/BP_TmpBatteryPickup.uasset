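; BP_TmpBatteryPickup is a temporary battery pickup that uses its transparent material to show whether it overlaps another actor.
; When an actor other than the player's ThirdPersonCharacter begins overlapping, PickupMesh swaps from TransparentBattery to Transparent_Collision_Battery.
; End overlap by such an actor swaps it back, without checking for other remaining overlaps.
; The current material acts as the state, so no variable tracks it.
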(event EventBeginPlay)

(event Collision|EventActorBeginOverlap
  (params (OtherActor :type Actor%20Object%20Reference))
  (bind _pickupmesh (Variables|Default|GetPickupMesh))
  (bind _asthird_person_character (Utilities|Casting|CastToThirdPersonCharacter (Game|GetPlayerCharacter 0)))
  (if (and (== (Rendering|Material|GetMaterial _pickupmesh 0) "/Game/Materials/TransparentBattery.TransparentBattery") (!= OtherActor _asthird_person_character))
    (Rendering|Material|SetMaterial _pickupmesh 0 "/Game/Materials/Transparent_Collision_Battery.Transparent_Collision_Battery")))

(event EventTick
  (params (DeltaSeconds :type Float%20%28single-precision%29)))

(event Collision|EventActorEndOverlap
  (params (OtherActor :type Actor%20Object%20Reference))
  (bind _asthird_person_character (Utilities|Casting|CastToThirdPersonCharacter (Game|GetPlayerCharacter 0)))
  (if (and (!= OtherActor _asthird_person_character) (== (Rendering|Material|GetMaterial (Variables|Default|GetPickupMesh) 0) "/Game/Materials/Transparent_Collision_Battery.Transparent_Collision_Battery"))
    (Rendering|Material|SetMaterial (Variables|Default|GetPickupMesh) 0 "/Game/Materials/TransparentBattery.TransparentBattery")))

(fn ConstructionScript)