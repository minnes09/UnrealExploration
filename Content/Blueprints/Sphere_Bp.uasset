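; Sphere actor that repeatedly emits randomly rotated laser-noise particle beams from its LaserEmit component, attached to the mesh's "center" socket.
; BeginPlay loops on a retriggerable delay, spawning a new attached emitter each pass and aiming it at a point scaled from the socket's world location.
; BeamCharge increments a counter, clearing its timer below 100 and switching to the LaserBeam template at 100, but nothing here calls it.
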(event EventBeginPlay
  (bind _laseremit (Variables|Default|GetLaserEmit))
  (bind _returnvalue (Transformation|GetSocketLocation _laseremit "None"))
  (Utilities|FlowControl|RetriggerableDelay (Variables|Default|GetCount%20Down%20Timer) :!label _label)
  (bind _returnvalue_2 (Effects|SpawnEmitterAttached "/Game/Beam/LaserBeamNoise.LaserBeamNoise" _laseremit "None" "0, 0, 0" (Math|Rotator|MakeRotator (Math|Random|RandomFloatinRange -1.8e+02 1.8e+02) (Math|Random|RandomFloatinRange -1.8e+02 1.8e+02) (Math|Random|RandomFloatinRange -1.8e+02 1.8e+02))))
  (Variables|Default|SetLaserTarget (+ _returnvalue (* _returnvalue 1000)))
  (Class|ParticleSystemComponent|SetBeamSourcePoint (Variables|Default|GetLaserEmit) 0 "0, 0, 0")
  (Class|ParticleSystemComponent|SetBeamTargetPoint _returnvalue_2 0 (Variables|Default|GetLaserTarget))
  (goto _label))

(event Collision|EventActorBeginOverlap
  (params (OtherActor :type Actor%20Object%20Reference)))

(fn ConstructionScript
  (Transformation|AttachComponentToComponent (Variables|Default|GetLaserEmit) (Variables|Debug|GetStaticMeshComponent) "center" "KeepRelative" "KeepRelative" "KeepRelative" true))

(fn BeamCharge
  (Variables|Default|SetIntBeamChargeRate (+ (Variables|Default|GetIntBeamChargeRate) 1))
  (if (!= (Variables|Default|GetIntBeamChargeRate) 100)
    (Utilities|Time|ClearTimerbyFunctionName 0 "BeamCharge")
    (else
      (Effects|Components|ParticleSystem|SetTemplate (Variables|Default|GetLaserEmit) "/Game/Beam/LaserBeam.LaserBeam"))))